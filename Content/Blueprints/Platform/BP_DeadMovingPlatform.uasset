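; BP_DeadMovingPlatform is a side-scroller platform that moves only while the player character is dead and overlapping its trigger box.
; On BeginPlay it adds a relative end point to its InterpToMovement, activates it, then disables the component's tick.
; Box overlaps toggle that tick, using IsCharacterAlive from SideScrollingGameInstance to allow movement.
; Actor Tick also polls that flag and freezes the platform whenever the character is alive.
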(event `self.ReceiveBeginPlay`
  (bind _interptomovement (`self.InterpToMovement`))
  (bind _asbp_side_scrolling_character (cast `/Game/Gamemode/BP_SideScrollingCharacter` (`GameplayStatics.GetPlayerCharacter` 0)))
  (set `self.As BP Side Scrolling Character` _asbp_side_scrolling_character)
  (`InterpToMovementComponent.AddControlPointPosition` _interptomovement (`self.EndRelativeLocation`) true)
  (`ActorComponent.Activate` _interptomovement false)
  (`ActorComponent.SetComponentTickEnabled` _interptomovement false))

(event `self.Box Collision.OnComponentBeginOverlap`
  (params (OverlappedComponent :type "PrimitiveComponent Object Reference") (OtherActor :type "Actor Object Reference") (OtherComp :type "PrimitiveComponent Object Reference") (OtherBodyIndex :type Integer) (bFromSweep :type Boolean) (SweepResult :type "HitResult Structure (by ref)"))
  (bind _asside_scrolling_game_instance (cast `SideScrollingGameInstance` (`GameplayStatics.GetGameInstance`)))
  (if (and (not (`SideScrollingGameInstance.bIsCharacterAlive` _asside_scrolling_game_instance)) (== OtherActor (`self.As BP Side Scrolling Character`)))
    (`ActorComponent.SetComponentTickEnabled` (`self.InterpToMovement`) true)))

(event `self.Box Collision.OnComponentEndOverlap`
  (params (OverlappedComponent :type "PrimitiveComponent Object Reference") (OtherActor :type "Actor Object Reference") (OtherComp :type "PrimitiveComponent Object Reference") (OtherBodyIndex :type Integer))
  (if (== OtherActor (`self.As BP Side Scrolling Character`))
    (`ActorComponent.SetComponentTickEnabled` (`self.InterpToMovement`) false)))

(event `self.ReceiveTick`
  (params (DeltaSeconds :type "Float (single-precision)"))
  (bind _asside_scrolling_game_instance (cast `SideScrollingGameInstance` (`GameplayStatics.GetGameInstance`)))
  (if (`SideScrollingGameInstance.bIsCharacterAlive` _asside_scrolling_game_instance)
    (`ActorComponent.SetComponentTickEnabled` (`self.InterpToMovement`) false)))

(fn `UserConstructionScript`)