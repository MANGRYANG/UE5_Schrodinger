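; Decorative cube that tumbles continuously on all three axes at a randomly varying speed.
; Two looping timers started on BeginPlay rapidly re-randomize per-axis frequency and amplitude.
; Each Tick adds local rotation to the mesh from the sine of frame delta times frequency, scaled by amplitude.
; Because the sine takes frame delta rather than elapsed time, the cube creeps in positive directions instead of oscillating.
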(event `self.ReceiveBeginPlay`
  (`KismetSystemLibrary.K2_SetTimer` null "SetRandomFreq" 0.01 true)
  (`KismetSystemLibrary.K2_SetTimer` null "SetRandomAmp" 0.01 true))

(event `self.ReceiveTick`
  (params (DeltaSeconds :type "Float (single-precision)"))
  (`SceneComponent.K2_AddLocalRotation` (`self.StaticMeshComponent`) (`KismetMathLibrary.MakeRotator` (* (`KismetMathLibrary.Sin` (* DeltaSeconds (`self.FreqX`))) (`self.AmpX`)) (* (`KismetMathLibrary.Sin` (* DeltaSeconds (`self.FreqY`))) (`self.AmpY`)) (* (`KismetMathLibrary.Sin` (* DeltaSeconds (`self.FreqZ`))) (`self.AmpZ`))) false false))

(fn `SetRandomAmp`
  (set `self.AmpX` (`KismetMathLibrary.RandomIntegerInRange` 10 15))
  (set `self.AmpY` (`KismetMathLibrary.RandomIntegerInRange` 10 15))
  (set `self.AmpZ` (`KismetMathLibrary.RandomIntegerInRange` 10 15)))

(fn `SetRandomFreq`
  (set `self.FreqX` (`KismetMathLibrary.RandomFloatInRange` 0.05 0.3))
  (set `self.FreqY` (`KismetMathLibrary.RandomFloatInRange` 0.05 0.3))
  (set `self.FreqZ` (`KismetMathLibrary.RandomFloatInRange` 0.05 0.3)))

(fn `UserConstructionScript`)