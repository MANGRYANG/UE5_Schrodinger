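; Box gimmick for a side-scrolling game that is passable or solid depending on whether the player character is alive or dead.
; When PlayerCheck begins an overlap, it reads IsCharacterAlive from SideScrollingGameInstance and compares it with the CanPassWhenPlayerIsAlive and CanPassWhenPlayerIsDead flags.
; The Cube's Pawn collision response then becomes Ignore or Block.
; The state updates only on overlap begin, with no filter on the overlapping actor.
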(event `self.PlayerCheck.OnComponentBeginOverlap`
  (params (OverlappedComponent :type "PrimitiveComponent Object Reference") (OtherActor :type "Actor Object Reference") (OtherComp :type "PrimitiveComponent Object Reference") (OtherBodyIndex :type Integer) (bFromSweep :type Boolean) (SweepResult :type "HitResult Structure (by ref)"))
  (bind _asside_scrolling_game_instance (cast `SideScrollingGameInstance` (`GameplayStatics.GetGameInstance`)))
  (if (or (and (`SideScrollingGameInstance.bIsCharacterAlive` _asside_scrolling_game_instance) (`self.Can Pass When Player Is Alive?`)) (and (not (`SideScrollingGameInstance.bIsCharacterAlive` _asside_scrolling_game_instance)) (`self.Can Pass When Player Is Dead?`)))
    (`PrimitiveComponent.SetCollisionResponseToChannel` (`self.Cube`) "ECC_Pawn" "ECR_Ignore")
    (else
      (`PrimitiveComponent.SetCollisionResponseToChannel` (`self.Cube`) "ECC_Pawn" "ECR_Block"))))

(fn `UserConstructionScript`)