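; BP_ObservationDrone is a drone gimmick that ends the game when its observation check succeeds.
; Every tick it calls StartObservation, which is defined outside this file, and a DoOnce lets the first true result through.
; That result plays a failure sound, calls GameOver on the SideScrollingGameInstance, shows a fade-out widget and opens GameOverMap after a short delay.
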(event `self.ReceiveTick`
  (params (DeltaSeconds :type "Float (single-precision)"))
  (bind _returnvalue (`self.StartObservation`))
  (if _returnvalue
    (`/Engine/EditorBlueprintResources/StandardMacros.DoOnce` false
      (:`Completed`
        (`GameplayStatics.PlaySound2D` "/Engine/EditorSounds/Notifications/CompileFailed_Cue.CompileFailed_Cue" 1.0 1.0 0.0 null null)
        (bind _asside_scrolling_game_instance (cast `SideScrollingGameInstance` (`GameplayStatics.GetGameInstance`)))
        (`SideScrollingGameInstance.GameOver` _asside_scrolling_game_instance)
        (bind _returnvalue_2 (`|CreateWidget` "/Game/Blueprints/WBP/WBP_FadeOut.WBP_FadeOut_C"))
        (`UserWidget.AddToViewport` _returnvalue_2 0)
        (`KismetSystemLibrary.Delay` 1.0)
        (`GameplayStatics.OpenLevel` "GameOverMap")))))

(fn `UserConstructionScript`)