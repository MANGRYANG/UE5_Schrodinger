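; BP_Ophanim is an Ophanim figure with four independently spinning rings and an animated eye.
; Each tick, every ring adds its own rotation step, blended between minimum and maximum speed by a repeating Gaussian curve over game time, producing periodic surges.
; Per-ring arrays set each curve and spin direction; steps are not scaled by delta time.
; The eye's world pitch and yaw sway together on a sine of time.
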(event `self.ReceiveTick`
  (params (DeltaSeconds :type "Float (single-precision)"))
  (bind _returnvalue (`GameplayStatics.GetTimeSeconds`))
  (`self.Rotate Ring` (`self.Ring`) 0 _returnvalue 8.0 0.5)
  (`self.Rotate Ring` (`self.Ring_001`) 1 _returnvalue 5.0 1.0)
  (`self.Rotate Ring` (`self.Ring_002`) 2 _returnvalue 6.0 4.0)
  (`self.Rotate Ring` (`self.Ring_003`) 3 _returnvalue 10.0 2.0)
  (`self.Rotate Eyeball` _returnvalue))

(fn `Probability Density Function`
  (params (Mu :type "Float (double-precision)") (Cycle :type "Float (double-precision)") (Sigma :type "Float (double-precision)") (xValue :type "Float (double-precision)"))
  (returns (Result :type "Float (double-precision)"))
  (return (* (`KismetMathLibrary.Exp` (* -0.5 (`KismetMathLibrary.Square` (* (- (mod xValue Cycle) Mu) (/ 1.0 Sigma))))) (/ 1.0 (* Sigma (`KismetMathLibrary.Sqrt` (`KismetMathLibrary.MultiplyByPi` 2.0)))))))

(fn `Rotate Eyeball`
  (params (`X Value` :type "Float (double-precision)"))
  (bind _returnvalue (`KismetMathLibrary.Lerp` 0.0 -10.0 (`KismetMathLibrary.Sin` `X Value`)))
  (`SceneComponent.K2_SetWorldRotation` (`self.Eye1`) (`KismetMathLibrary.MakeRotator` 0.0 _returnvalue _returnvalue) false false))

(fn `Rotate Ring`
  (params (TargetRing :type "StaticMeshComponent Object Reference") (Index :type Integer) (`Time Second` :type "Float (double-precision)") (`Max Speed` :type "Float (double-precision)") (`Min Speed` :type "Float (double-precision)"))
  (locals (idx :type Integer) (Max :type "Float (double-precision)") (Min :type "Float (double-precision)"))
  (bind _idx (`local.idx`))
  (set `local.Max` `Max Speed`)
  (set `local.Min` `Min Speed`)
  (set `local.idx` Index)
  (bind _result (`self.Probability Density Function` (`|GetArrayItem` (`self.Mu`) _idx) (`|GetArrayItem` (`self.Cycle`) _idx) (`|GetArrayItem` (`self.Sigma`) _idx) `Time Second`))
  (`SceneComponent.K2_SetWorldRotation` TargetRing (`KismetMathLibrary.ComposeRotators` (`SceneComponent.K2_GetComponentRotation` TargetRing) (* (`|GetArrayItem` (`self.RotateDirection`) (`local.idx`)) (`KismetMathLibrary.Lerp` (`local.Min`) (`local.Max`) _result))) true false))

(fn `UserConstructionScript`)