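; BP_Eleonore is an NPC Blueprint that opens a dialog with the player when they are close enough.
; Overlap begin and end events on CommunicationCollision toggle a flag allowing communication, without filtering which actor overlaps.
; While the flag is set, the IA_Communicate Enhanced Input action creates WBP_Dialog, adds it to the viewport and switches to UI-only input with a locked mouse.
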(event `self.Communication Collision.OnComponentBeginOverlap`
  (params (OverlappedComponent :type "PrimitiveComponent Object Reference") (OtherActor :type "Actor Object Reference") (OtherComp :type "PrimitiveComponent Object Reference") (OtherBodyIndex :type Integer) (bFromSweep :type Boolean) (SweepResult :type "HitResult Structure (by ref)"))
  (set `self.Can Player Communicate With Eleonore?` true))

(event `self.Communication Collision.OnComponentEndOverlap`
  (params (OverlappedComponent :type "PrimitiveComponent Object Reference") (OtherActor :type "Actor Object Reference") (OtherComp :type "PrimitiveComponent Object Reference") (OtherBodyIndex :type Integer))
  (set `self.Can Player Communicate With Eleonore?` false))

(event `EnhancedInput|/Game/Input/IA_Communicate`
  (params (ActionValue :type Boolean) (ElapsedSeconds :type "Float (double-precision)") (TriggeredSeconds :type "Float (double-precision)") (InputAction :type "InputAction Object Reference" :default "/Game/Input/IA_Communicate.IA_Communicate"))
  (:`Started`
    (if (`self.Can Player Communicate With Eleonore?`)
      (bind _returnvalue (`|CreateWidget` "/Game/Blueprints/WBP/WBP_Dialog.WBP_Dialog_C" (`GameplayStatics.GetPlayerController` 0)))
      (`UserWidget.AddToViewport` _returnvalue 0)
      (`WidgetBlueprintLibrary.SetInputMode_UIOnlyEx` (`GameplayStatics.GetPlayerController` 0) _returnvalue "LockAlways"))))

(fn `UserConstructionScript`)