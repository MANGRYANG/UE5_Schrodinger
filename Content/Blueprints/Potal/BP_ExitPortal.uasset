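; BP_ExitPortal is a level exit portal that sends the player to the game-clear map.
; A box overlap toggles whether the player is on the portal, without checking which actor overlapped.
; Pressing the portal input while that flag is set disables player input, plays an eject sound, shows a fade-out widget, then opens GameClearMap after a short delay.
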(event `self.Box.OnComponentBeginOverlap`
  (params (OverlappedComponent :type "PrimitiveComponent Object Reference") (OtherActor :type "Actor Object Reference") (OtherComp :type "PrimitiveComponent Object Reference") (OtherBodyIndex :type Integer) (bFromSweep :type Boolean) (SweepResult :type "HitResult Structure (by ref)"))
  (set `self.Is Player On Portal?` true))

(event `self.Box.OnComponentEndOverlap`
  (params (OverlappedComponent :type "PrimitiveComponent Object Reference") (OtherActor :type "Actor Object Reference") (OtherComp :type "PrimitiveComponent Object Reference") (OtherBodyIndex :type Integer))
  (set `self.Is Player On Portal?` false))

(event `EnhancedInput|/Game/Input/IA_Portal`
  (params (ActionValue :type Boolean) (ElapsedSeconds :type "Float (double-precision)") (TriggeredSeconds :type "Float (double-precision)") (InputAction :type "InputAction Object Reference" :default "/Game/Input/IA_Portal.IA_Portal"))
  (bind _returnvalue (`GameplayStatics.GetPlayerController` 0))
  (:`Started`
    (if (`self.Is Player On Portal?`)
      (`self.DisableInput` (`GameplayStatics.GetPlayerCharacter` 0) _returnvalue)
      (`GameplayStatics.PlaySound2D` "/Engine/EditorSounds/GamePreview/EjectFromPlayer_Cue.EjectFromPlayer_Cue" 1.0 1.0 0.0 null null)
      (bind _returnvalue_2 (`|CreateWidget` "/Game/Blueprints/WBP/WBP_FadeOut.WBP_FadeOut_C" _returnvalue))
      (`UserWidget.AddToViewport` _returnvalue_2 0)
      (`KismetSystemLibrary.Delay` 0.6)
      (`GameplayStatics.OpenLevel` "GameClearMap"))))

(fn `UserConstructionScript`)