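; A one-way platform that the player can jump up through from below and drop down through from on top.
; CollisionBottom overlaps toggle the Platform's collision off on entry and back on at exit, for the player character only.
; CollisionTop tracks whether the player stands on the platform, letting the IA_PlayerDown input disable collision for a drop.
; After a drop, collision returns only when the player leaves CollisionBottom.
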(event `self.Collision Bottom.OnComponentBeginOverlap`
  (params (OverlappedComponent :type "PrimitiveComponent Object Reference") (OtherActor :type "Actor Object Reference") (OtherComp :type "PrimitiveComponent Object Reference") (OtherBodyIndex :type Integer) (bFromSweep :type Boolean) (SweepResult :type "HitResult Structure (by ref)"))
  ; Collision settings for jumping over the platform
  (if (== OtherActor (`GameplayStatics.GetPlayerCharacter` 0))
    (`PrimitiveComponent.SetCollisionEnabled` (`self.Platform`) "NoCollision")))

(event `self.Collision Bottom.OnComponentEndOverlap`
  (params (OverlappedComponent :type "PrimitiveComponent Object Reference") (OtherActor :type "Actor Object Reference") (OtherComp :type "PrimitiveComponent Object Reference") (OtherBodyIndex :type Integer))
  ; Collision settings for jumping over the platform
  (if (== OtherActor (`GameplayStatics.GetPlayerCharacter` 0))
    (`PrimitiveComponent.SetCollisionEnabled` (`self.Platform`) "QueryAndPhysics")))

(event `self.Collision Top.OnComponentBeginOverlap`
  (params (OverlappedComponent :type "PrimitiveComponent Object Reference") (OtherActor :type "Actor Object Reference") (OtherComp :type "PrimitiveComponent Object Reference") (OtherBodyIndex :type Integer) (bFromSweep :type Boolean) (SweepResult :type "HitResult Structure (by ref)"))
  ; Set the Boolean variable to see if the player is on the platform
  (if (== OtherActor (`GameplayStatics.GetPlayerCharacter` 0))
    (set `self.Is On Top Of Platform?` true)))

(event `self.Collision Top.OnComponentEndOverlap`
  (params (OverlappedComponent :type "PrimitiveComponent Object Reference") (OtherActor :type "Actor Object Reference") (OtherComp :type "PrimitiveComponent Object Reference") (OtherBodyIndex :type Integer))
  ; Set the Boolean variable to see if the player is on the platform
  (if (== OtherActor (`GameplayStatics.GetPlayerCharacter` 0))
    (set `self.Is On Top Of Platform?` false)))

(event `EnhancedInput|/Game/Input/IA_PlayerDown`
  (params (ActionValue :type Boolean) (ElapsedSeconds :type "Float (double-precision)") (TriggeredSeconds :type "Float (double-precision)") (InputAction :type "InputAction Object Reference" :default "/Game/Input/IA_PlayerDown.IA_PlayerDown"))
  ; Allow Player to drop down through platform
  (:`Started`
    (if (`self.Is On Top Of Platform?`)
      (`PrimitiveComponent.SetCollisionEnabled` (`self.Platform`) "NoCollision"))))

(fn `UserConstructionScript`)